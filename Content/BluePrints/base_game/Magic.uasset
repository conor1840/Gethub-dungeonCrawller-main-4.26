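; Magic is a spell actor with a hitbox that damages AI characters and bursts in an explosion effect.
; On overlap with an AI_Base, a DoOnce gate applies damage and burn, spawns the explosion at the hitbox and destroys the actor.
; Tick also polls the player FPS_char's ToggleFire and, when true, explodes and destroys the actor after a short delay.
; An older Dummy_AI damage path is left unconnected.
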(event `self.ReceiveTick`
  (params (DeltaSeconds :type "Float (single-precision)"))
  (bind _magic_hitbox (`self.Magic Hitbox`))
  (bind _returnvalue (+ (`SceneComponent.K2_GetComponentLocation` _magic_hitbox) (`KismetMathLibrary.GreaterGreater_VectorRotator` (0.0 0.0 0.0) (`SceneComponent.K2_GetComponentRotation` _magic_hitbox))))
  (`|ExecutionSequence`
    (:`then_0`
      (bind _asfps_char (cast `/Game/BluePrints/base_game/FPS_char` (`GameplayStatics.GetPlayerCharacter` 0)))
      (if (`/Game/BluePrints/base_game/FPS_char.Toggle Fire ` _asfps_char)
        (`KismetSystemLibrary.Delay` 0.5)
        (`GameplayStatics.SpawnEmitterAtLocation` "/Game/FXVarietyPack/Particles/P_ky_explosion.P_ky_explosion" _returnvalue (`KismetMathLibrary.Conv_VectorToRotator` _returnvalue))
        (`self.K2_DestroyActor`)))))

(event `self.Magic Hitbox.OnComponentBeginOverlap`
  (params (OverlappedComponent :type "PrimitiveComponent Object Reference") (OtherActor :type "Actor Object Reference") (OtherComp :type "PrimitiveComponent Object Reference") (OtherBodyIndex :type Integer) (bFromSweep :type Boolean) (SweepResult :type "HitResult Structure (by ref)"))
  (bind _magic_hitbox (`self.Magic Hitbox`))
  (bind _returnvalue (+ (`SceneComponent.K2_GetComponentLocation` _magic_hitbox) (`KismetMathLibrary.GreaterGreater_VectorRotator` (0.0 0.0 0.0) (`SceneComponent.K2_GetComponentRotation` _magic_hitbox))))
  (bind _asai_base (cast `/Game/BluePrints/AI/Meele/AI_Base` OtherActor))
  (`/Engine/EditorBlueprintResources/StandardMacros.DoOnce` false :!label _label
    (:`Completed`
      (`/Game/BluePrints/AI/Meele/AI_Base.TakeDamage` _asai_base 25)
      (`/Game/BluePrints/AI/Meele/AI_Base.Burn Damge` _asai_base)
      (`GameplayStatics.SpawnEmitterAtLocation` "/Game/FXVarietyPack/Particles/P_ky_explosion.P_ky_explosion" _returnvalue (`KismetMathLibrary.Conv_VectorToRotator` _returnvalue))
      (`self.K2_DestroyActor`)
      (goto _label :!via `Reset`))))

(fn `UserConstructionScript`)