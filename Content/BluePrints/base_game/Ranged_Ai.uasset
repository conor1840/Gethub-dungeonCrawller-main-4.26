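; Ranged_Ai is a ranged enemy that turns to face the player and repeatedly fires AI_Magic actors.
; Each Tick casts the player character to FPS_char and snaps the actor's rotation toward it, with no range or line-of-sight check.
; A Delay on Tick throttles spawning to roughly every two seconds.
; Projectiles spawn at the Box component's location and rotation, as the intended forward offset is zero.
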(event `self.ReceiveTick`
  (params (DeltaSeconds :type "Float (single-precision)"))
  (bind _box (`self.Box`))
  (bind _returnvalue (`SceneComponent.K2_GetComponentRotation` _box))
  (bind _asfps_char (cast `/Game/BluePrints/base_game/FPS_char` (`GameplayStatics.GetPlayerCharacter` 0)))
  (`self.K2_SetActorRotation` (`KismetMathLibrary.FindLookAtRotation` (`self.K2_GetActorLocation`) (`self.K2_GetActorLocation` _asfps_char)))
  (`KismetSystemLibrary.Delay` 2.0)
  (`|SpawnActorFromClass` "/Game/BluePrints/base_game/AI_Magic.AI_Magic_C" (`KismetMathLibrary.MakeTransform` (+ (`SceneComponent.K2_GetComponentLocation` _box) (`KismetMathLibrary.GreaterGreater_VectorRotator` (0.0 0.0 0.0) _returnvalue)) _returnvalue) "Undefined" "OverrideRootScale" null null))

(fn `UserConstructionScript`)