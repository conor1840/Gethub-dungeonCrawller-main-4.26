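; Chest actor that spins in the world and can be opened by the player, disappearing afterward.
; Tick applies a frame-rate-independent yaw rotation driven by RotateSpeed.
; The ChestOpen custom event checks IsChestOpen on the FPS_char player, plays the Chest_open montage at reduced speed on the skeletal mesh, then destroys the actor when it completes.
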(event `self.ReceiveTick`
  (params (DeltaSeconds :type "Float (single-precision)"))
  (`self.K2_AddActorLocalRotation` (* (`KismetMathLibrary.MakeRotator` 0.0 0.0 (`self.Rotate Speed`)) DeltaSeconds)))

(event `Chest Open`
  (bind _asfps_char (cast `/Game/BluePrints/base_game/FPS_char` (`GameplayStatics.GetPlayerCharacter` 0)))
  (if (`/Game/BluePrints/base_game/FPS_char.Is chest open` _asfps_char)
    (`|PlayMontage` (`self.SkeletalMesh`) "/Game/Meshes/Chest/Chest_open.Chest_open" 0.5
      (:`OnCompleted`
        (`self.K2_DestroyActor`)))))

(fn `UserConstructionScript`)