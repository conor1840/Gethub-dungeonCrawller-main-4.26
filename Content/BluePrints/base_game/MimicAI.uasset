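; Mimic enemy actor that acts as a one-shot trap when the FPS player character enters its box trigger.
; Each overlap calls the open animation, then immediately starts the looping idle with no delay, replacing it.
; A DoOnce with no reset limits it to a single hit of damage on the player.
; Tick is empty, and a leftover rotation node never runs.
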(event `self.Box.OnComponentBeginOverlap`
  (params (OverlappedComponent :type "PrimitiveComponent Object Reference") (OtherActor :type "Actor Object Reference") (OtherComp :type "PrimitiveComponent Object Reference") (OtherBodyIndex :type Integer) (bFromSweep :type Boolean) (SweepResult :type "HitResult Structure (by ref)"))
  (bind _asfps_char (cast `/Game/BluePrints/base_game/FPS_char` OtherActor))
  (`|ExecutionSequence`
    (:`then_0`
      (`SkeletalMeshComponent.PlayAnimation` (`self.SkeletalMesh`) "/Game/Meshes/Mimic/Mimic_Open.Mimic_Open" false)
      (`SkeletalMeshComponent.PlayAnimation` (`self.SkeletalMesh`) "/Game/Meshes/Mimic/NPC_Mimic_Anim_Root_Mimic_Idle.NPC_Mimic_Anim_Root_Mimic_Idle" true))
    (:`then_1`
      (`/Engine/EditorBlueprintResources/StandardMacros.DoOnce` false
        (:`Completed`
          (`/Game/BluePrints/base_game/FPS_char.TakeDamage` _asfps_char 1.0))))))

(event `self.ReceiveTick`
  (params (DeltaSeconds :type "Float (single-precision)")))

(fn `UserConstructionScript`)