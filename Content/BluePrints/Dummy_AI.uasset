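; Dummy AI actor with an AIHealth value that takes burn damage over time.
; BurnDamge sets a looping one-second timer on itself and decrements health on each call, while a DoOnce-gated delay pauses the timer after five seconds and resets the gate.
; Tick prints health for debugging and destroys the actor only when DeltaSeconds equals zero, with no check on AIHealth.
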(event `self.ReceiveTick`
  (params (DeltaSeconds :type "Float (single-precision)"))
  (`|ExecutionSequence`
    (:`then_0`
      (if (== DeltaSeconds 0.0)
        (`self.K2_DestroyActor`)))
    (:`then_1`
      (`KismetSystemLibrary.PrintString` (`KismetStringLibrary.Conv_DoubleToString` (`self.AI Health`))))))

(event `Burn Damge`
  (bind _returnvalue (`KismetSystemLibrary.K2_SetTimerDelegate` (delegate `Burn Damge`) 1.0 true))
  (set `self.AI Health` (- (`self.AI Health`) 1.0))
  (`/Engine/EditorBlueprintResources/StandardMacros.DoOnce` false :!label _label
    (:`Completed`
      (`KismetSystemLibrary.Delay` 5.0)
      (`KismetSystemLibrary.K2_PauseTimerHandle` _returnvalue)
      (goto _label :!via `Reset`))))

(fn `UserConstructionScript`)