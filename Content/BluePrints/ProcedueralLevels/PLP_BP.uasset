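; Procedural level room that chains the next room and populates its own encounter for the FPS character.
; Leaving the Entracne trigger moves the door, spawns three AI enemies, a chest and a CombatDirector given the enemy list.
; The Exit trigger spawns Level_4 when NumberOfLevels is 3, otherwise randomly Level_1 or Level_2, then destroys this room after a delay.
; Re-rolled random checks can spawn nothing and never reach Level_3.
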(event `self.ReceiveBeginPlay`
  (set `self.SpawnPoints` (`|MakeArray` (`self.SpawnPoint`) (`self.SpawnPoint1`) (`self.SpawnPoint2`) (`self.SpawnPoint3`) (`self.SpawnPoint4`) (`self.SpawnPoint5`)))
  (set `self.Levels` (`self.GetAllChildActors` true)))

(event `self.Exit.OnComponentBeginOverlap`
  (params (OverlappedComponent :type "PrimitiveComponent Object Reference") (OtherActor :type "Actor Object Reference") (OtherComp :type "PrimitiveComponent Object Reference") (OtherBodyIndex :type Integer) (bFromSweep :type Boolean) (SweepResult :type "HitResult Structure (by ref)"))
  (cast `/Game/BluePrints/base_game/FPS_char` OtherActor)
  (`/Engine/EditorBlueprintResources/StandardMacros.DoOnce` false :!label _label
    (:`Completed`
      (if (== (`self.Number of levels`) 3)
        (`KismetSystemLibrary.PrintString` "end")
        (`|SpawnActorFromClass` "/Game/BluePrints/ProcedueralLevels/PLP_BP_Level_4.PLP_BP_Level_4_C" (`SceneComponent.K2_GetComponentToWorld` (`self.NextRoomSpawn`)) "Undefined" "OverrideRootScale" null self null)
        (elif (== (`KismetMathLibrary.RandomInteger` 2) 0)
          (`KismetSystemLibrary.PrintString` "first")
          (`|SpawnActorFromClass` "/Game/BluePrints/ProcedueralLevels/PLP_BP_Level_1.PLP_BP_Level_1_C" (`SceneComponent.K2_GetComponentToWorld` (`self.NextRoomSpawn`)) "Undefined" "OverrideRootScale" null self null)
          (set `self.Preivous Level` self :!label _label_2)
          (bind _output_get (set `self.Number of levels` (+ 1 (`self.Number of levels`))))
          (`KismetSystemLibrary.PrintString` (`KismetStringLibrary.Conv_IntToString` _output_get))
          (`KismetSystemLibrary.Delay` 5.0)
          (`self.K2_DestroyActor` (`self.Preivous Level`))
          (goto _label :!via `Reset`)
          (elif (== (`KismetMathLibrary.RandomInteger` 2) 1)
            (`KismetSystemLibrary.PrintString` "second")
            (`|SpawnActorFromClass` "/Game/BluePrints/ProcedueralLevels/PLP_BP_Level_2.PLP_BP_Level_2_C" (`SceneComponent.K2_GetComponentToWorld` (`self.NextRoomSpawn`)) "Undefined" "OverrideRootScale" null self null)
            (goto _label_2)
            (elif (== (`KismetMathLibrary.RandomInteger` 2) 2)
              (`KismetSystemLibrary.PrintString` "third")
              (`|SpawnActorFromClass` "/Game/BluePrints/ProcedueralLevels/PLP_BP_Level_3.PLP_BP_Level_3_C" (`SceneComponent.K2_GetComponentToWorld` (`self.NextRoomSpawn`)) "Undefined" "OverrideRootScale" null self null)
              (goto _label_2))))))))

(event `self.Entracne.OnComponentEndOverlap`
  (params (OverlappedComponent :type "PrimitiveComponent Object Reference") (OtherActor :type "Actor Object Reference") (OtherComp :type "PrimitiveComponent Object Reference") (OtherBodyIndex :type Integer))
  (cast `/Game/BluePrints/base_game/FPS_char` OtherActor)
  (`SceneComponent.K2_SetRelativeLocation` (`self.Door`) (0.0 0.0 110.0) false false)
  (bind _returnvalue (`|SpawnActorFromClass` "/Game/BluePrints/AI/Meele/CombatDirector.CombatDirector_C" (`SceneComponent.K2_GetComponentToWorld` (`self.SpawnPoint4`)) "Undefined" "OverrideRootScale" null null))
  (set `self.CombatDirector` _returnvalue)
  (`|SpawnActorFromClass` "/Game/BluePrints/AI/Meele/AI_Base.AI_Base_C" (`SceneComponent.K2_GetComponentToWorld` (`self.SpawnPoint`)) "Undefined" "OverrideRootScale" null null)
  (`|SpawnActorFromClass` "/Game/BluePrints/AI/Meele/AI_Base.AI_Base_C" (`SceneComponent.K2_GetComponentToWorld` (`self.SpawnPoint1`)) "Undefined" "OverrideRootScale" null null)
  (`|SpawnActorFromClass` "/Game/BluePrints/AI/Meele/AI_Base.AI_Base_C" (`SceneComponent.K2_GetComponentToWorld` (`self.SpawnPoint2`)) "Undefined" "OverrideRootScale" null null)
  (`|SpawnActorFromClass` "/Game/BluePrints/base_game/Chest.Chest_C" (`SceneComponent.K2_GetComponentToWorld` (`self.SpawnPoint5`)) "Undefined" "OverrideRootScale" null null)
  (set `/Game/BluePrints/AI/Meele/CombatDirector.EnemyList` (`|MakeArray` null null null :!type "/Game/BluePrints/AI/Meele/AI_Base Object Reference") (`self.CombatDirector`)))

(fn `UserConstructionScript`)